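; Course spline actor that generates pairs of angled side splines along its length from the construction script.
; GenerateSideSplines spawns two new course spline actors at fixed distance intervals, swapping their "main" tag for the passed tag and yawing their splines to opposite sides.
; Each side spline is offset and shaped into a short curve sized by the parent spline's local scale, with point scales growing along it.
; RegenerateZones is an empty stub.
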(event EventBeginPlay)

(event Collision|EventActorBeginOverlap
  (params (OtherActor :type Actor%20Object%20Reference)))

(event EventTick
  (params (DeltaSeconds :type Float%20%28single-precision%29)))

(fn ConstructionScript
  (CallFunction|GenerateSideSplines "None"))

(fn GenerateSideSplines
  (params (tag :type Name))
  (bind _spline (Variables|Default|GetSpline))
  (for _index (range 0 (Math|Float|Truncate (/ (Spline|GetSplineLength _spline) 2e+03)))
    (for _index_2 (range 0 1)
      (bind _returnvalue (Game|SpawnActorfromClass "BP_CourseSpline_C" (Math|Transform|MakeTransform (.location (Spline|GetTransformatDistanceAlongSpline _spline (* (Math|Conversions|ToFloat(Integer) _index) 2e+03) "World" true)) (.rotation (Spline|GetTransformatDistanceAlongSpline _spline (* (Math|Conversions|ToFloat(Integer) _index) 2e+03) "World" true)) "1.000000,1.000000,1.000000") "Undefined" "MultiplyWithRoot" 0 0))
      (Utilities|Array|RemoveItem (Variables|/Script/Engine.Actor|GetTags _returnvalue) "main")
      (Utilities|Array|Add (Variables|/Script/Engine.Actor|GetTags _returnvalue) tag)
      (Variables|/Script/Engine.Actor|SetTags _returnvalue (Variables|/Script/Engine.Actor|GetTags _returnvalue))
      (Transformation|AddLocalRotation (Actor|GetComponentbyClass _returnvalue "/Script/Engine.SplineComponent") (Math|Rotator|MakeRotator 0.0 0.0 (Utilities|Select :Index _index_2 :Option%200 45.0 :Option%201 -45.0)) false false)
      (Transformation|AddLocalOffset (Actor|GetComponentbyClass _returnvalue "/Script/Engine.SplineComponent") (* (Math|Vector|MakeVector (* (Math|Float|Max(Float) (.X (Math|Vector|BreakVector (.scale (Spline|GetTransformatDistanceAlongSpline _spline (* (Math|Conversions|ToFloat(Integer) _index) 2e+03) "World" true)))) (.Y (Math|Vector|BreakVector (.scale (Spline|GetTransformatDistanceAlongSpline _spline (* (Math|Conversions|ToFloat(Integer) _index) 2e+03) "World" true)))) (.Z (Math|Vector|BreakVector (.scale (Spline|GetTransformatDistanceAlongSpline _spline (* (Math|Conversions|ToFloat(Integer) _index) 2e+03) "World" true))))) 3e+02) 0.0 0.0) -1.0) false false)
      (Spline|SetLocationatSplinePoint (Actor|GetComponentbyClass _returnvalue "/Script/Engine.SplineComponent") 1 (Math|Vector|MakeVector (* (Math|Float|Max(Float) (.X (Math|Vector|BreakVector (.scale (Spline|GetTransformatDistanceAlongSpline _spline (* (Math|Conversions|ToFloat(Integer) _index) 2e+03) "World" true)))) (.Y (Math|Vector|BreakVector (.scale (Spline|GetTransformatDistanceAlongSpline _spline (* (Math|Conversions|ToFloat(Integer) _index) 2e+03) "World" true)))) (.Z (Math|Vector|BreakVector (.scale (Spline|GetTransformatDistanceAlongSpline _spline (* (Math|Conversions|ToFloat(Integer) _index) 2e+03) "World" true))))) 1e+02) (Utilities|Select :Index _index_2 :Option%200 2e+02 :Option%201 -2e+02) 0.0) "Local" true)
      (Spline|AddSplinePoint (Actor|GetComponentbyClass _returnvalue "/Script/Engine.SplineComponent") (Math|Vector|MakeVector (* (Math|Float|Max(Float) (.X (Math|Vector|BreakVector (.scale (Spline|GetTransformatDistanceAlongSpline _spline (* (Math|Conversions|ToFloat(Integer) _index) 2e+03) "World" true)))) (.Y (Math|Vector|BreakVector (.scale (Spline|GetTransformatDistanceAlongSpline _spline (* (Math|Conversions|ToFloat(Integer) _index) 2e+03) "World" true)))) (.Z (Math|Vector|BreakVector (.scale (Spline|GetTransformatDistanceAlongSpline _spline (* (Math|Conversions|ToFloat(Integer) _index) 2e+03) "World" true))))) 3e+02) 0.0 0.0) "Local" true)
      (for _index_3 (range 0 2)
        (Class|SplineComponent|SetScaleatSplinePoint (Actor|GetComponentbyClass _returnvalue "/Script/Engine.SplineComponent") _index_3 (/ (.scale (Spline|GetTransformatDistanceAlongSpline _spline (* (Math|Conversions|ToFloat(Integer) _index) 2e+03) "World" true)) (Utilities|Select :Index _index_3 :Option%200 4.0 :Option%201 3.0 :Option%202 2.0)) true)))))

(fn RegenerateZones)