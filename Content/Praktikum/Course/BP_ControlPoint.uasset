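; Course control point that rides the main BP_CourseSpline, trailing its ControlTarget by a set distance along the spline.
; When LockPos is set it stops moving and runs CalcCone, deriving rubberband strength from the target's angle against a forward cone.
; Strength rises toward the cone edge and beyond, and InCone is true whenever it is above zero.
; Construction scales the cone to half-angle and length and snaps the actor to the spline.
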(event EventBeginPlay)

(event EventTick
  (params (DeltaSeconds :type Float%20%28single-precision%29))
  (bind _disttoplayer (Variables|Default|GetdistToPlayer))
  (bind _spline (Variables|Default|Getspline))
  (bind _spline_2 (Variables|Default|Getspline))
  (bind _controltarget (Variables|Default|GetcontrolTarget))
  (bind _returnvalue (Transformation|GetActorLocation _controltarget))
  (bind _returnvalue_2 (* _disttoplayer 1e+02))
  (bind _returnvalue_3 (Class|SplineComponent|FindInputKeyClosesttoWorldLocation _spline _returnvalue))
  (bind _returnvalue_4 (Class|SplineComponent|GetDistanceAlongSplineatSplineInputKey _spline _returnvalue_3))
  (bind _returnvalue_5 (- _returnvalue_4 _returnvalue_2))
  (bind _returnvalue_6 (Spline|GetTransformatDistanceAlongSpline _spline_2 _returnvalue_5 "World" false))
  (Utilities|IsValid _controltarget
    (:Is%20Valid
      (if (!= (Variables|Default|GetlockPos) true)
        (Transformation|SetActorLocationAndRotation (.location _returnvalue_6) (.rotation _returnvalue_6))
        (else
          (CallFunction|CalcCone))))))

(fn ConstructionScript
  (bind _halfangledeg (Variables|Default|GethalfAngleDeg))
  (bind _length (Variables|Default|Getlength))
  (bind _returnvalue (Math|Trig|DegreesToRadians _halfangledeg))
  (bind _returnvalue_2 (Math|Trig|Tan(Radians) _returnvalue))
  (bind _returnvalue_3 (* _returnvalue_2 _length))
  (Utilities|FlowControl|Sequence
    (:then_0
      (Transformation|SetWorldScale3D (Variables|Default|GetunitCone) (Math|Vector|MakeVector _returnvalue_3 _returnvalue_3 _length)))
    (:then_1
      (bind _outactors (Actor|GetAllActorsOfClasswithTag "/Game/Praktikum/Course/BP_CourseSpline.BP_CourseSpline_C" "main"))
      (Variables|Default|Setspline (Actor|GetComponentbyClass (Utilities|Array|Get(acopy) _outactors) "/Script/Engine.SplineComponent"))
      (Variables|Default|SetcurrentDistance (Class|SplineComponent|GetDistanceAlongSplineatSplineInputKey (Variables|Default|Getspline) (Class|SplineComponent|FindInputKeyClosesttoWorldLocation (Variables|Default|Getspline) (Transformation|GetActorLocation))))
      (Transformation|SetActorTransform (Class|SplineComponent|GetTransformatSplineInputKey (Variables|Default|Getspline) (Class|SplineComponent|FindInputKeyClosesttoWorldLocation (Variables|Default|Getspline) (Transformation|GetActorLocation)) "World" false)))))

(fn CalcCone
  (bind _returnvalue (Transformation|GetActorLocation))
  (bind _returnvalue_2 (Transformation|GetActorForwardVector))
  (bind _controltarget (Variables|Default|GetcontrolTarget))
  (bind _halfangledeg (Variables|Default|GethalfAngleDeg))
  (bind _returnvalue_3 (Math|Trig|Cos(Degrees) _halfangledeg))
  (bind _returnvalue_4 (Transformation|GetActorLocation _controltarget))
  (bind _returnvalue_5 (Math|Rotator|FindLookatRotation _returnvalue _returnvalue_4))
  (bind _returnvalue_6 (Math|Vector|GetForwardVector _returnvalue_5))
  (bind _returnvalue_7 (Math|Vector|DotProduct _returnvalue_2 _returnvalue_6))
  (bind _returnvalue_8 (- _returnvalue_7 _returnvalue_3))
  (bind _returnvalue_9 (* _returnvalue_8 1e+01))
  (bind _returnvalue_10 (Math|Float|Clamp(Float) _returnvalue_9))
  (bind _returnvalue_11 (- 1.0 _returnvalue_10))
  (return _returnvalue_11 (> _returnvalue_11 0.0)))