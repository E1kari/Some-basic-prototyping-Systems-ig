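; BP_DragTrigger is a trigger volume that hands the player character over to a spline-based drag rail.
; On actor overlap, it gets the course spline and control point from its linked DragPoint and passes them to the player's SplineMode.
; It then enters the player into a "Rail" zone.
; The construction script sizes the sphere from TriggerRadius and aims and stretches an arrow to show the link to the DragPoint.
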(event EventBeginPlay)

(event Collision|EventActorBeginOverlap
  (params (OtherActor :type Actor%20Object%20Reference))
  (bind _asbp_player_character (Utilities|Casting|CastToBP_PlayerCharacter OtherActor))
  (bind _asbp_course_spline (Utilities|Casting|CastToBP_CourseSpline (Components|GetOwner (Variables|/Game/Praktikum/Course/BP_DragPoint.BP_DragPoint_C|GetMetadata%20Spline (Variables|Default|GetdragPoint)))))
  (bind _control_point (Default|GetControlPointonSpline (Variables|Default|GetdragPoint)))
  (Default|EnterDragTrigger (Variables|/Game/Praktikum/Player/BP_PlayerCharacter.BP_PlayerCharacter_C|GetsplineMode _asbp_player_character) (Variables|Default|GetdragPoint) _asbp_course_spline _control_point)
  (Default|EnterZone _asbp_player_character "Rail" 0.0 "0, 0, 0"))

(event EventTick
  (params (DeltaSeconds :type Float%20%28single-precision%29)))

(fn ConstructionScript
  (bind _returnvalue (Transformation|GetActorLocation))
  (bind _dragpoint (Variables|Default|GetdragPoint))
  (bind _arrow (Variables|Default|GetArrow))
  (bind _returnvalue_2 (Transformation|GetActorLocation _dragpoint))
  (Utilities|FlowControl|Sequence
    (:then_0
      (Components|Sphere|SetSphereRadius (Variables|Default|GetSphere) (Variables|Default|GettriggerRadius) false))
    (:then_1
      (Transformation|SetWorldRotation _arrow (Math|Rotator|FindLookatRotation _returnvalue _returnvalue_2) false false)
      (Variables|/Script/Engine.ArrowComponent|SetArrowLength _arrow (Math|Vector|Distance(Vector) _returnvalue _returnvalue_2)))))