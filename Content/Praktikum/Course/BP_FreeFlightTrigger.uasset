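; BP_FreeFlightTrigger is a spherical trigger volume that puts the player into the FreeFlight zone.
; On actor overlap it casts to BP_PlayerCharacter and calls EnterZone with zero strength and direction; it has no end-overlap handling.
; The construction script sizes the sphere from TriggerRadius and sets an arrow's rotation and length using the actor's own location as both start and target, giving it zero length.
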(event EventBeginPlay)

(event Collision|EventActorBeginOverlap
  (params (OtherActor :type Actor%20Object%20Reference))
  (bind _asbp_player_character (Utilities|Casting|CastToBP_PlayerCharacter OtherActor))
  (Default|EnterZone _asbp_player_character "FreeFlight" 0.0 "0, 0, 0"))

(event EventTick
  (params (DeltaSeconds :type Float%20%28single-precision%29)))

(fn ConstructionScript
  (bind _returnvalue (Transformation|GetActorLocation))
  (bind _returnvalue_2 (Transformation|GetActorLocation))
  (bind _arrow (Variables|Default|GetArrow))
  (Utilities|FlowControl|Sequence
    (:then_0
      (Components|Sphere|SetSphereRadius (Variables|Default|GetSphere) (Variables|Default|GettriggerRadius) false))
    (:then_1
      (Transformation|SetWorldRotation _arrow (Math|Rotator|FindLookatRotation _returnvalue_2 _returnvalue) false false)
      (Variables|/Script/Engine.ArrowComponent|SetArrowLength _arrow (Math|Vector|Distance(Vector) _returnvalue_2 _returnvalue)))))