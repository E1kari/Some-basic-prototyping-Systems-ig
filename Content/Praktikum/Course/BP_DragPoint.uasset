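; BP_DragPoint is a rail attractor that snaps to the nearest BP_CourseSpline and hands the player to spline mode with that spline's control point.
; Magnet and Trigger sphere overlaps set the Magnet or Active state, which selects pull strength; leaving Magnet deactivates it if detaching is allowed.
; While engaged, Tick keeps the actor a set distance ahead of the player along the spline, with both spheres following the player's closest spline point.
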(event OnComponentBeginOverlap(Trigger)
  (params (OverlappedComponent :type Primitive%20Component%20Object%20Reference) (OtherActor :type Actor%20Object%20Reference) (OtherComp :type Primitive%20Component%20Object%20Reference) (OtherBodyIndex :type Integer) (bFromSweep :type Boolean) (SweepResult :type Hit%20Result%20Structure%20%28by%20ref%29))
  (bind _asbp_player_character (Utilities|Casting|CastToBP_PlayerCharacter OtherActor))
  (Variables|Default|Setstate "NewEnumerator2")
  (CallFunction|EnterTrigger _asbp_player_character)
  (Default|EnterZone _asbp_player_character "Rail" 0.0 "0, 0, 0")
  (Variables|Default|SetdragTarget _asbp_player_character)
  (Default|UpdateMagnetisation (Variables|/Game/Praktikum/Player/BP_PlayerCharacter.BP_PlayerCharacter_C|GetsplineMode _asbp_player_character)))

(event OnComponentBeginOverlap(Magnet)
  (params (OverlappedComponent :type Primitive%20Component%20Object%20Reference) (OtherActor :type Actor%20Object%20Reference) (OtherComp :type Primitive%20Component%20Object%20Reference) (OtherBodyIndex :type Integer) (bFromSweep :type Boolean) (SweepResult :type Hit%20Result%20Structure%20%28by%20ref%29))
  (bind _asbp_player_character (Utilities|Casting|CastToBP_PlayerCharacter OtherActor))
  (Variables|Default|Setstate "NewEnumerator1")
  (Default|EnterZone _asbp_player_character "Rail" 0.0 "0, 0, 0")
  (Variables|Default|SetdragTarget _asbp_player_character)
  (Utilities|IsValid (Variables|/Game/Praktikum/Player/PlayerModes/splineMode.splineMode_C|Getspline (Variables|/Game/Praktikum/Player/BP_PlayerCharacter.BP_PlayerCharacter_C|GetsplineMode _asbp_player_character))
    (:Is%20Valid
      _)
    (:Is%20Not%20Valid
      (CallFunction|EnterTrigger _asbp_player_character)))
  (Default|UpdateMagnetisation (Variables|/Game/Praktikum/Player/BP_PlayerCharacter.BP_PlayerCharacter_C|GetsplineMode _asbp_player_character)))

(event OnComponentEndOverlap(Trigger)
  (params (OverlappedComponent :type Primitive%20Component%20Object%20Reference) (OtherActor :type Actor%20Object%20Reference) (OtherComp :type Primitive%20Component%20Object%20Reference) (OtherBodyIndex :type Integer)))

(event OnComponentEndOverlap(Magnet)
  (params (OverlappedComponent :type Primitive%20Component%20Object%20Reference) (OtherActor :type Actor%20Object%20Reference) (OtherComp :type Primitive%20Component%20Object%20Reference) (OtherBodyIndex :type Integer))
  (bind _asbp_player_character (Utilities|Casting|CastToBP_PlayerCharacter OtherActor))
  (bind _allowedtodetach (Default|AllowedtoDetach (Variables|/Game/Praktikum/Player/BP_PlayerCharacter.BP_PlayerCharacter_C|GetsplineMode (Variables|Default|GetdragTarget)) "NewEnumerator1"))
  (if _allowedtodetach
    (Variables|Default|Setstate "NewEnumerator0")
    (Default|UpdateMagnetisation (Variables|/Game/Praktikum/Player/BP_PlayerCharacter.BP_PlayerCharacter_C|GetsplineMode _asbp_player_character))))

(event EventBeginPlay
  (CallFunction|Init))

(event EventTick
  (params (DeltaSeconds :type Float%20%28single-precision%29))
  (bind _metadata_spline (Variables|Default|GetMetadata%20Spline))
  (bind _disttoplayer (Variables|Default|GetdistToPlayer))
  (bind _metadata_spline_2 (Variables|Default|GetMetadata%20Spline))
  (bind _metadata_spline_3 (Variables|Default|GetMetadata%20Spline))
  (bind _dragtarget (Variables|Default|GetdragTarget))
  (bind _returnvalue (Transformation|GetActorLocation _dragtarget))
  (bind _returnvalue_2 (* _disttoplayer 1e+02))
  (bind _returnvalue_3 (Class|SplineComponent|FindInputKeyClosesttoWorldLocation _metadata_spline _returnvalue))
  (bind _returnvalue_4 (Class|SplineComponent|GetDistanceAlongSplineatSplineInputKey _metadata_spline _returnvalue_3))
  (bind _returnvalue_5 (Spline|GetTransformatDistanceAlongSpline _metadata_spline_2 _returnvalue_4 "World" false))
  (bind _returnvalue_6 (+ _returnvalue_2 _returnvalue_4))
  (bind _returnvalue_7 (Spline|GetTransformatDistanceAlongSpline _metadata_spline_3 _returnvalue_6 "World" false))
  (if (Utilities|Enum|NotEqual(Enum) (Variables|Default|Getstate) "NewEnumerator0")
    (Utilities|IsValid _dragtarget
      (:Is%20Valid
        (Utilities|FlowControl|Sequence
          (:then_0
            (Transformation|SetActorLocationAndRotation (.location _returnvalue_7) (.rotation _returnvalue_7)))
          (:then_1
            (Transformation|SetWorldLocationAndRotation (Variables|Default|GetMagnet) (.location _returnvalue_5) (.rotation _returnvalue_5) false false)))))))

(event EventOnMoveFinishedinEditor
  (CallFunction|Init))

(fn ConstructionScript)

(fn LookatStrenght
  (return (Math|Float|Clamp(Float) (Math|Vector|DotProduct (Math|Vector|GetForwardVector (Variables|/Game/Praktikum/Player/BP_PlayerCharacter.BP_PlayerCharacter_C|GetBox (Variables|Default|GetdragTarget))) (Math|Vector|GetForwardVector (Math|Rotator|FindLookatRotation (Transformation|GetActorLocation (Variables|Default|GetdragTarget)) (Transformation|GetActorLocation)))))))

(fn UpdateNearestSpline
  (bind _returnvalue (Transformation|GetActorLocation))
  (LocalVariables|SetlowestDist -1.0)
  (bind _outactors (Actor|GetAllActorsOfClass "/SplinePointsMetadata/BP_CourseSpline.BP_CourseSpline_C"))
  (for (_array_element _array_index) _outactors
    (Rendering|Debug|DrawDebugLine "0, 0, 0" "0, 0, 0" (select (or (< (Math|Vector|Distance(Vector) _returnvalue (.location (Class|SplineComponent|FindTransformClosesttoWorldLocation (Variables|/SplinePointsMetadata/BP_CourseSpline.BP_CourseSpline_C|GetMetadataSpline _array_element) _returnvalue "World" false))) (LocalVariables|GetlowestDist)) (== (LocalVariables|GetlowestDist) -1.0)) "(R=0.059272,G=0.598958,B=0.142360,A=1.000000)" "(R=0.744792,G=0.050429,B=0.050429,A=1.000000)") 0.0 0.0)
    (if (or (< (Math|Vector|Distance(Vector) _returnvalue (.location (Class|SplineComponent|FindTransformClosesttoWorldLocation (Variables|/SplinePointsMetadata/BP_CourseSpline.BP_CourseSpline_C|GetMetadataSpline _array_element) _returnvalue "World" false))) (LocalVariables|GetlowestDist)) (== (LocalVariables|GetlowestDist) -1.0))
      (LocalVariables|SetclosestIndex _array_index)
      (LocalVariables|SetlowestDist (Math|Vector|Distance(Vector) _returnvalue (.location (Class|SplineComponent|FindTransformClosesttoWorldLocation (Variables|/SplinePointsMetadata/BP_CourseSpline.BP_CourseSpline_C|GetMetadataSpline _array_element) _returnvalue "World" false))))))
  (Variables|Default|SetMetadata%20Spline (Variables|/SplinePointsMetadata/BP_CourseSpline.BP_CourseSpline_C|GetMetadataSpline (Utilities|Array|Get(acopy) _outactors (LocalVariables|GetclosestIndex)))))

(fn GetControlPointonSpline
  (bind _metadata_spline (Variables|Default|GetMetadata%20Spline))
  (bind _outactors (Actor|GetAllActorsOfClass "/Game/Praktikum/Course/BP_ControlPoint.BP_ControlPoint_C"))
  (for _array_element _outactors
    (if (and (Utilities|IsValid (Variables|/Game/Praktikum/Course/BP_ControlPoint.BP_ControlPoint_C|GetMetadata%20Spline _array_element)) (Utilities|IsValid _metadata_spline))
      (if (== (Components|GetOwner (Variables|/Game/Praktikum/Course/BP_ControlPoint.BP_ControlPoint_C|GetMetadata%20Spline _array_element)) (Components|GetOwner _metadata_spline))
        (bind _output_get (Variables|Default|SetcontrolPoint _array_element))
        (return _output_get)))))

(fn Init
  (bind _returnvalue (Transformation|GetActorLocation))
  (bind _returnvalue_2 (Utilities|FindDistanceAlongSplineClosesttoWorldLocation _returnvalue))
  (Utilities|FlowControl|Sequence
    (:then_0
      (CallFunction|UpdateNearestSpline)
      (CallFunction|GetControlPointonSpline)
      (LocalVariables|Setraw%20dist _returnvalue_2)
      (Transformation|SetActorTransform (Spline|GetTransformatDistanceAlongSpline (Variables|Default|GetMetadata%20Spline) (+ _returnvalue_2 (Variables|Default|GetdistToPlayer)) "World" false)))
    (:then_1
      (Components|Sphere|SetSphereRadius (Variables|Default|GetMagnet) (* (Variables|Default|GetmagnetRadius) 1e+02) false)
      (Components|Sphere|SetSphereRadius (Variables|Default|GetTrigger) (* (Variables|Default|GettriggerRadius) 1e+02) false)
      (Transformation|SetWorldLocationAndRotation (Variables|Default|GetMagnet) (.location (Spline|GetTransformatDistanceAlongSpline (Variables|Default|GetMetadata%20Spline) (LocalVariables|Getraw%20dist) "World" false)) (.rotation (Spline|GetTransformatDistanceAlongSpline (Variables|Default|GetMetadata%20Spline) (LocalVariables|Getraw%20dist) "World" false)) false false))))

(fn ActivateSplineMode
  (params (InputPin :type BP%20Player%20Character%20Object%20Reference))
  (bind _asbp_course_spline (Utilities|Casting|CastToBP_CourseSpline (Components|GetOwner (Variables|Default|GetMetadata%20Spline))))
  (bind _control_point (CallFunction|GetControlPointonSpline self))
  (Default|EnterDragTrigger (Variables|/Game/Praktikum/Player/BP_PlayerCharacter.BP_PlayerCharacter_C|GetsplineMode InputPin) _control_point _asbp_course_spline self)
  (Default|EnterZone InputPin "Rail" 0.0 "0, 0, 0")
  (Variables|Default|SetdragTarget InputPin))

(fn GetPullStrenght
  (return (Utilities|Select :Index (Variables|Default|Getstate) :NewEnumerator0 0.0 :NewEnumerator1 (Variables|Default|GetmagnetStrenght) :NewEnumerator2 (Variables|Default|GetactiveStrenght))))

(fn EnterTrigger
  (params (dragTarget :type BP%20Player%20Character%20Object%20Reference))
  (bind _asbp_course_spline (Utilities|Casting|CastToBP_CourseSpline (Components|GetOwner (Variables|Default|GetMetadata%20Spline))))
  (bind _control_point (CallFunction|GetControlPointonSpline self))
  (Default|EnterDragTrigger (Variables|/Game/Praktikum/Player/BP_PlayerCharacter.BP_PlayerCharacter_C|GetsplineMode dragTarget) _control_point _asbp_course_spline self))