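; Flight camera controller component that reads camera state from its owning actor through BPI_CameraStateProvider.
; On BeginPlay it checks that the owner implements the interface, printing an error if not.
; Each Tick it caches the provider's camera state message; no camera is adjusted here.
; A debug function, not called in these graphs, prints the cached in-thermal flag.
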(event EventBeginPlay
  (Init|ResolveStateProvider))

(event EventTick
  (params (DeltaSeconds :type Float%20%28single-precision%29))
  (Init|RefreshCameraState))

(fn ResolveStateProvider
  (bind _returnvalue (Components|GetOwner))
  (bind _output_get (Variables|Default|SetbHasValidProvider (Utilities|DoesObjectImplementInterface _returnvalue "/Game/Praktikum/Camera/BPI_CameraStateProvider.BPI_CameraStateProvider_C")))
  (if _output_get
    (Variables|Default|SetStateProviderActor _returnvalue)
    (else
      (Development|PrintString "BP_AC_FlightCameraController: No valid provider" true true "(R=0.578125,G=0.000000,B=0.079457,A=1.000000)" 5.0))))

(fn RefreshCameraState
  (if (Variables|Default|GetbHasValidProvider)
    (bind _camerastate (Class|BPICameraStateProvider|GetCameraState(Message) (Variables|Default|GetStateProviderActor)))
    (Variables|Default|SetCachedCameraState _camerastate)))

(fn DebugDrawCameraState
  (params (DeltaTime :type Float%20%28double-precision%29))
  (Development|PrintString (Utilities|String|Append "Is In Thermal: " " " (Utilities|String|ToString(Boolean) (.bisinthermal (Variables|Default|GetCachedCameraState)))) true true "(R=0.000000,G=0.075578,B=1.000000,A=1.000000)" DeltaTime))