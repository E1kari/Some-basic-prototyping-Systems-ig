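; Player flight-mode Blueprint that provides movement, visual banking and airspeed functions for the jet plane player character.
; ExecuteMovement pushes along camera forward with slight input steering while boosting, otherwise rotates the character's Box with clamped pitch, and returns whether boost applied.
; OrientPlane interpolates the jet mesh toward input-driven roll and pitch.
; UpdateAirspeed gains speed in dives and loses it in climbs within limits; the camera-state function is an empty stub.
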(event EventBeginPlay)

(event EventTick
  (params (DeltaSeconds :type Float%20%28single-precision%29)))

(fn OrientPlane
  (params (PlayerCharacter :type BP%20Player%20Character%20Object%20Reference) (Input :type Rotator))
  (bind (_roll _pitch _yaw) (Math|Rotator|BreakRotator Input))
  (bind _jet_plane (Variables|/Game/Praktikum/Player/BP_PlayerCharacter.BP_PlayerCharacter_C|GetJet_Plane PlayerCharacter))
  (Transformation|SetRelativeRotation _jet_plane (Math|Interpolation|RInterpTo (Variables|/Script/Engine.SceneComponent|GetRelativeRotation _jet_plane) (Math|Rotator|MakeRotator (* _yaw (Variables|Default|GetMaxVisualRollAngle)) (* (Variables|Default|GetMaxVisualPitchAngle) _pitch) 0.0) (Utilities|Time|GetWorldDeltaSeconds) (Variables|Default|GetInterpolationSpeed)) false false))

(fn ExecuteMovement
  (params (PlayerCharacter :type BP%20Player%20Character%20Object%20Reference) (Input :type Rotator))
  (bind _playercharacter (LocalVariables|GetplayerCharacter))
  (bind _maxpitchangle (Variables|Default|GetMaxPitchAngle))
  (bind (_roll _pitch _yaw) (Math|Rotator|BreakRotator Input))
  (bind (_roll_2 _pitch_2 _yaw_2) (Math|Rotator|BreakRotator Input))
  (bind _box (Variables|/Game/Praktikum/Player/BP_PlayerCharacter.BP_PlayerCharacter_C|GetBox PlayerCharacter))
  (bind _relativerotation (Variables|/Script/Engine.SceneComponent|GetRelativeRotation _box))
  (if (Utilities|Enum|Equal(Enum) (Variables|/Game/Praktikum/Player/BP_PlayerCharacter.BP_PlayerCharacter_C|Getboosting PlayerCharacter) "Active")
    ;[0.15 0.15 0.15 0.5] boost
    (Pawn|Input|AddMovementInput _playercharacter (Math|Vector|GetForwardVector (Variables|/Game/Praktikum/Player/BP_PlayerCharacter.BP_PlayerCharacter_C|GetCamera (LocalVariables|GetplayerCharacter))) 1.0 false)
    (Pawn|Input|AddMovementInput _playercharacter (Math|Vector|MakeVector _yaw 0.0 _pitch) 0.25 false)
    (return true)
    (else
      ;[0.15 0.15 0.15 0.5] default
      (Transformation|SetRelativeRotation (Variables|/Game/Praktikum/Player/BP_PlayerCharacter.BP_PlayerCharacter_C|GetBox PlayerCharacter) (Math|Rotator|MakeRotator (+ _roll_2 (.roll _relativerotation)) (Math|Float|Clamp(Float) (+ _pitch_2 (.pitch _relativerotation)) (* -1.0 _maxpitchangle) _maxpitchangle) (+ _yaw_2 (.yaw _relativerotation))) false false)
      (return false))))

(fn UpdateAirspeed
  (params (deltaSeconds :type Float%20%28double-precision%29) (Input :type Rotator))
  (bind _floatingpawnvalues (Variables|DesignerVariable|PresetValue|GetFloatingPawnValues))
  (Utilities|FlowControl|Sequence
    (:then_0
      ;[0.15 0.15 0.15 0.5] Extra speed because of dive
      (bind _output_get (LocalVariables|SetTempDive (Math|Float|Clamp(Float) (* (.pitch Input) -1.0))))
      (LocalVariables|SetDiveSpeedDelta (* _output_get (Variables|DesignerVariable|NoseDip/Climbing|GetDiveAccel) deltaSeconds)))
    (:then_1
      ;[0.15 0.15 0.15 0.5] Reduced speed because of climbing
      (bind _output_get_2 (LocalVariables|SetTempPull (Math|Float|Clamp(Float) (.pitch Input))))
      (LocalVariables|SetPullSpeedDelta (* _output_get_2 (Variables|DesignerVariable|NoseDip/Climbing|GetPullUpDecel) deltaSeconds)))
    (:then_2
      ;[0.15 0.15 0.15 0.5] Update Airspeed
      (Variables|Internal|SetAirSpeed (Math|Float|Clamp(Float) (- (+ (Variables|Internal|GetAirSpeed) (LocalVariables|GetDiveSpeedDelta)) (LocalVariables|GetPullSpeedDelta)) (.minairspeed _floatingpawnvalues) (.maxairspeed _floatingpawnvalues))))
    (:then_3
      (return (LocalVariables|GetTempDive) (LocalVariables|GetTempPull)))))

(fn ReAppendCameraStateData
  (params (InData :type ST%20Camera%20State%20Structure))
  (return ""))