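; BP_ThermalVolume is a thermal updraft zone that lifts the player character inside its capsule.
; Capsule overlaps register and unregister the volume with BP_PlayerCharacter.
; While the player is inside, Tick sends the character a lift rate for this thermal.
; The rate uses horizontal distance from the center, peaking at MaxLiftRate and falling to zero at the capsule radius along a FalloffPower curve.
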(event OnComponentBeginOverlap(Capsule)
  (params (OverlappedComponent :type Primitive%20Component%20Object%20Reference) (OtherActor :type Actor%20Object%20Reference) (OtherComp :type Primitive%20Component%20Object%20Reference) (OtherBodyIndex :type Integer) (bFromSweep :type Boolean) (SweepResult :type Hit%20Result%20Structure%20%28by%20ref%29))
  ;[0.15 0.15 0.15 0.5] Subscribe this thermal volume to the player
  (bind _asbp_player_character (Utilities|Casting|CastToBP_PlayerCharacter OtherActor))
  (bind _output_get (Variables|DontTouch|BackgroundValue|SetPlayerCharacter _asbp_player_character))
  (Default|RegisterThermal _output_get self)
  (Variables|DontTouch|BackgroundValue|SetbPlayerInside true))

(event OnComponentEndOverlap(Capsule)
  (params (OverlappedComponent :type Primitive%20Component%20Object%20Reference) (OtherActor :type Actor%20Object%20Reference) (OtherComp :type Primitive%20Component%20Object%20Reference) (OtherBodyIndex :type Integer))
  ;[0.15 0.15 0.15 0.5] Unsub this thermal volume from the player
  (if (== OtherActor (Variables|DontTouch|BackgroundValue|GetPlayerCharacter))
    (Default|UnregisterThermal (Variables|DontTouch|BackgroundValue|GetPlayerCharacter) self)
    (Variables|DontTouch|BackgroundValue|SetbPlayerInside false)))

(event EventTick
  (params (DeltaSeconds :type Float%20%28single-precision%29))
  (bind _playercharacter (Variables|DontTouch|BackgroundValue|GetPlayerCharacter))
  ;[0.15 0.15 0.15 0.5] Update the strength of the thermal volume in the player
  (if (Variables|DontTouch|BackgroundValue|GetbPlayerInside)
    (Default|UpdateThermalLift _playercharacter self (CallFunction|CalculateLiftStrength _playercharacter))))

(fn ConstructionScript)

(fn CalculateLiftStrength
  (params (Player :type BP%20Player%20Character%20Object%20Reference))
  (return (* (Math|Float|Power (- 1.0 (Math|Float|Clamp(Float) (/ (Math|Vector|Distance2D(Vector) (Transformation|GetActorLocation) (Transformation|GetActorLocation Player)) (Variables|/Script/Engine.CapsuleComponent|GetCapsuleRadius (Variables|Default|GetCapsule))))) (Variables|DesignerVariable|Lift|GetFalloffPower)) (Variables|DesignerVariable|Lift|GetMaxLiftRate))))