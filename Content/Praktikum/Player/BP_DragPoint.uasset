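; BP_DragPoint is an actor that travels along the "main" course spline, pacing itself against the tagged player character.
; BeginPlay caches the spline and player.
; Each Tick scales its step by MinSpeed, delta time and MaxDistance minus player distance in meters, slowing as the gap grows and reversing beyond the maximum.
; It accumulates CurrentDistance to set location and rotation from the spline, and prints the remaining margin for debugging.
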(event EventBeginPlay
  (bind _outactors (Actor|GetAllActorsOfClasswithTag "/Game/Praktikum/Course/BP_CourseSpline.BP_CourseSpline_C" "main"))
  (Variables|Default|Setspline (Utilities|Array|Get(acopy) _outactors))
  (bind _outactors_2 (Actor|GetAllActorsOfClasswithTag "/Game/Praktikum/Player/BP_PlayerCharacter.BP_PlayerCharacter_C" "Player"))
  (Variables|Default|Settarget (Utilities|Array|Get(acopy) _outactors_2)))

(event Collision|EventActorBeginOverlap
  (params (OtherActor :type Actor%20Object%20Reference)))

(event EventTick
  (params (DeltaSeconds :type Float%20%28single-precision%29))
  (bind _target (Variables|Default|Gettarget))
  (bind _maxdistance (Variables|Default|GetmaxDistance))
  (bind _returnvalue (Transformation|GetDistanceTo _target))
  (bind _returnvalue_2 (/ _returnvalue 1e+02))
  (bind _returnvalue_3 (- _maxdistance _returnvalue_2))
  (Utilities|IsValid _target
    (:Is%20Valid
      (Development|PrintString (Utilities|String|ToString(Float) _returnvalue_3))
      (Transformation|SetActorLocationAndRotation (.location (Spline|GetTransformatDistanceAlongSpline (Actor|GetComponentbyClass (Variables|Default|Getspline) "/Script/Engine.SplineComponent") (+ (* _returnvalue_3 (* DeltaSeconds (Variables|Default|GetminSpeed))) (Variables|Default|GetcurrentDistance)) "World" false)) (.rotation (Spline|GetTransformatDistanceAlongSpline (Actor|GetComponentbyClass (Variables|Default|Getspline) "/Script/Engine.SplineComponent") (+ (* _returnvalue_3 (* DeltaSeconds (Variables|Default|GetminSpeed))) (Variables|Default|GetcurrentDistance)) "World" false)))
      (Variables|Default|SetcurrentDistance (+ (* _returnvalue_3 (* DeltaSeconds (Variables|Default|GetminSpeed))) (Variables|Default|GetcurrentDistance))))))

(fn ConstructionScript)