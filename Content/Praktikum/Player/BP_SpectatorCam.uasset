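; BP_SpectatorCam is a spectator camera actor that hovers a set Distance above the player character, following its position and yaw.
; BeginPlay targets the first BP_PlayerCharacter found, and Tick searches again whenever that target is invalid.
; UpdatePosRot copies the target's location and yaw every tick, adding the height offset.
; An OnMoveFinishedinEditor event snaps it above the first PlayerStart instead, apparently as an editor preview.
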(event EventBeginPlay
  (bind _outactors (Actor|GetAllActorsOfClass "/Game/Praktikum/Player/BP_PlayerCharacter.BP_PlayerCharacter_C"))
  (Variables|Default|SetfollowTarget (Utilities|Array|Get(acopy) _outactors))
  (CallFunction|UpdatePos&Rot))

(event Collision|EventActorBeginOverlap
  (params (OtherActor :type Actor%20Object%20Reference)))

(event EventTick
  (params (DeltaSeconds :type Float%20%28single-precision%29))
  (Utilities|IsValid (Variables|Default|GetfollowTarget)
    (:Is%20Valid
      _)
    (:Is%20Not%20Valid
      (bind _outactors (Actor|GetAllActorsOfClass "/Game/Praktikum/Player/BP_PlayerCharacter.BP_PlayerCharacter_C"))
      (Variables|Default|SetfollowTarget (Utilities|Array|Get(acopy) _outactors))))
  (CallFunction|UpdatePos&Rot))

(event EventOnMoveFinishedinEditor
  (bind _outactors (Actor|GetAllActorsOfClass "/Script/Engine.PlayerStart"))
  (Variables|Default|SetfollowTarget (Utilities|Array|Get(acopy) _outactors))
  (CallFunction|UpdatePos&Rot))

(fn ConstructionScript)

(fn UpdatePos&Rot
  (bind _followtarget (Variables|Default|GetfollowTarget))
  (bind _returnvalue (Transformation|GetActorTransform _followtarget))
  (bind (_x _y _z) (Math|Vector|BreakVector (.location _returnvalue)))
  (Transformation|SetActorTransform (Math|Transform|MakeTransform (Math|Vector|MakeVector _x _y (+ _z (Variables|Default|Getdistance))) (Math|Rotator|MakeRotator 0.0 0.0 (.yaw (.rotation _returnvalue))) "1.000000,1.000000,1.000000")))