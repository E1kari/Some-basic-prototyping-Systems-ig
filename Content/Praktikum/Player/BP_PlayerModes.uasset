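; BP_PlayerModes provides flight movement and visual tilt functions that act on a passed-in player character with a jet plane.
; ExecuteMovement adds rotation input to the character's Box, clamping pitch to a symmetric limit.
; OrientPlane interpolates the JetPlane's relative rotation toward input-scaled maximum angles, turning yaw input into visual banking roll.
; The event graph is empty, so neither function is driven from within this Blueprint.
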(event EventBeginPlay)

(event EventTick
  (params (DeltaSeconds :type Float%20%28single-precision%29)))

(fn OrientPlane
  (params (PlayerCharacter :type BP%20Player%20Character%20Object%20Reference) (Input :type Rotator))
  (bind (_roll _pitch _yaw) (Math|Rotator|BreakRotator Input))
  (bind _jet_plane (Variables|/Game/Praktikum/Player/BP_PlayerCharacter.BP_PlayerCharacter_C|GetJet_Plane PlayerCharacter))
  (Transformation|SetRelativeRotation _jet_plane (Math|Interpolation|RInterpTo (Variables|/Script/Engine.SceneComponent|GetRelativeRotation _jet_plane) (Math|Rotator|MakeRotator (* _yaw (Variables|Default|GetMaxVisualRollAngle)) (* (Variables|Default|GetMaxVisualPitchAngle) _pitch) 0.0) (Utilities|Time|GetWorldDeltaSeconds) (Variables|Default|GetInterpolationSpeed)) false false))

(fn ExecuteMovement
  (params (PlayerCharacter :type BP%20Player%20Character%20Object%20Reference) (Input :type Rotator))
  (bind _box (Variables|/Game/Praktikum/Player/BP_PlayerCharacter.BP_PlayerCharacter_C|GetBox PlayerCharacter))
  (bind _maxpitchangle (Variables|Default|GetMaxPitchAngle))
  (bind _relativerotation (Variables|/Script/Engine.SceneComponent|GetRelativeRotation _box))
  (Transformation|SetRelativeRotation (Variables|/Game/Praktikum/Player/BP_PlayerCharacter.BP_PlayerCharacter_C|GetBox PlayerCharacter) (Math|Rotator|MakeRotator (+ (.roll _relativerotation) (.roll Input)) (Math|Float|Clamp(Float) (+ (.pitch Input) (.pitch _relativerotation)) (* -1.0 _maxpitchangle) _maxpitchangle) (+ (.yaw _relativerotation) (.yaw Input))) false false))